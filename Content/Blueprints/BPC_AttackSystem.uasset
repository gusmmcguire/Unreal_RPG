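; Actor component that runs a four-step melee combo (sword attacks plus a kick) on the BP_ThirdPersonCharacter mesh.
; IA_Attack starts a swing when CanAttack is set, or buffers the press in SaveAttack while already attacking.
; SwordAttackCombo, not called within this graph, either consumes that buffer to play the next step or calls StopCombo to reset.
; AttackIndex selects each montage, which plays after a short delay behind a DoOnce guard.
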(event Custom|Sword%20Attack
  ;[0.05098 0.05098 0.05098] Sword Attack
  (if (Variables|Default|GetIsAttacking)
    (Variables|Default|SetSaveAttack true)
    (else
      (Variables|Default|SetIsAttacking true)
      (switch int (Variables|Default|GetAttackIndex)
        (:0
          (CallFunction|Attack1))
        (:1
          (CallFunction|Attack2))
        (:2
          (CallFunction|Attack3))
        (:3
          (CallFunction|Attack4))))))

(event Custom|Sword%20Attack%20Combo
  ;[0.05098 0.05098 0.05098] Combo Continue
  (if (Variables|Default|GetSaveAttack)
    (Variables|Default|SetSaveAttack false)
    (switch int (Variables|Default|GetAttackIndex)
      (:0
        (CallFunction|Attack1))
      (:1
        (CallFunction|Attack2))
      (:2
        (CallFunction|Attack3))
      (:3
        (CallFunction|Attack4)))
    (else
      (CallFunction|StopCombo))))

(event Custom|Attack%202
  ;[0.05098 0.05098 0.05098] Attack 2
  (Utilities|FlowControl|DoOnce false :!label _label
    (:Completed
      (Utilities|FlowControl|Delay 0.2)
      (Animation|Montage|PlayMontage (Variables|Default|GetCharacterMesh) "/Game/Characters/RPG_Character/Animations/SwordAttacks/Attack2_Montage.Attack2_Montage"
        (:then
          (Variables|Default|SetAttackIndex 2)
          (goto _label Reset))))))

(event Custom|Attack%203
  ;[0.05098 0.05098 0.05098] Attack 3 (Kick Anim)
  (Utilities|FlowControl|DoOnce false :!label _label
    (:Completed
      (Utilities|FlowControl|Delay 0.2)
      (Animation|Montage|PlayMontage (Variables|Default|GetCharacterMesh) "/Game/Characters/RPG_Character/Animations/SwordAttacks/Kick_Montage.Kick_Montage"
        (:then
          (Variables|Default|SetAttackIndex 3)
          (goto _label Reset))))))

(event Custom|Stop%20Combo
  ;[0.05098 0.05098 0.05098] Stop Combo/Attack
  (Variables|Default|SetIsAttacking false)
  (Variables|Default|SetAttackIndex 0))

(event Custom|Attack%204
  ;[0.05098 0.05098 0.05098] Attack 4 (Attack 3 Anim)
  (Utilities|FlowControl|DoOnce false :!label _label
    (:Completed
      (Utilities|FlowControl|Delay 0.2)
      (Animation|Montage|PlayMontage (Variables|Default|GetCharacterMesh) "/Game/Characters/RPG_Character/Animations/SwordAttacks/Attack3_Montage.Attack3_Montage"
        (:then
          (Variables|Default|SetAttackIndex 4)
          (goto _label Reset))))))

(event Custom|Attack%201
  ;[0.05098 0.05098 0.05098] Attack 1
  (Utilities|FlowControl|DoOnce false :!label _label
    (:Completed
      (Utilities|FlowControl|Delay 0.2)
      (Animation|Montage|PlayMontage (Variables|Default|GetCharacterMesh) "/Game/Characters/RPG_Character/Animations/SwordAttacks/Attack1_Montage.Attack1_Montage"
        (:then
          (Variables|Default|SetAttackIndex 1)
          (goto _label Reset))))))

(event Input|EnhancedActionEvents|EnhancedInputActionIA_Attack
  (params (ActionValue :type Boolean) (ElapsedSeconds :type Float%20%28double-precision%29) (TriggeredSeconds :type Float%20%28double-precision%29) (InputAction :type Input%20Action%20Object%20Reference :default "/Game/ThirdPerson/Input/Actions/IA_Attack.IA_Attack"))
  ;[0.05098 0.05098 0.05098] Attack Input
  (:Started
    (if (Variables|Default|GetCanAttack)
      (CallFunction|SwordAttack))))

(event EventBeginPlay
  ;[0.05098 0.05098 0.05098] Get Character Mesh
  (bind _asbp_third_person_character (Utilities|Casting|CastToBP_ThirdPersonCharacter (Components|GetOwner)))
  (Variables|Default|SetCharacterMesh (Variables|/Script/Engine.Character|GetMesh _asbp_third_person_character)))