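; BP_Dummy is an assassination target that plays the victim side of a paired knife stealth kill from behind.
; An overlap radius toggles the assassinate prompt as the third-person character enters or leaves.
; StealthBackAssassin plays the victim montage and returns a reference location and the dummy's rotation for the attacker.
; It also triggers Ragdoll, which uses timed delays to play a death sound, then enable mesh physics.
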(event OnComponentBeginOverlap(AssassinationRadius)
  (params (OverlappedComponent :type Primitive%20Component%20Object%20Reference) (OtherActor :type Actor%20Object%20Reference) (OtherComp :type Primitive%20Component%20Object%20Reference) (OtherBodyIndex :type Integer) (bFromSweep :type Boolean) (SweepResult :type Hit%20Result%20Structure%20%28by%20ref%29))
  ;[0.05098 0.05098 0.05098] Handle Prompt Visibility
  (Utilities|Casting|CastToBP_ThirdPersonCharacter OtherActor)
  (Rendering|SetVisibility (Variables|Default|GetAssassinatePrompt) true false))

(event OnComponentEndOverlap(AssassinationRadius)
  (params (OverlappedComponent :type Primitive%20Component%20Object%20Reference) (OtherActor :type Actor%20Object%20Reference) (OtherComp :type Primitive%20Component%20Object%20Reference) (OtherBodyIndex :type Integer))
  ;[0.05098 0.05098 0.05098] Handle Prompt Visibility
  (Utilities|Casting|CastToBP_ThirdPersonCharacter OtherActor)
  (Rendering|SetVisibility (Variables|Default|GetAssassinatePrompt) false false))

(event Custom|Ragdoll
  ;[0.05098 0.05098 0.05098] Ragdoll
  (Utilities|FlowControl|Sequence
    (:then_0
      (Utilities|FlowControl|Delay 2.0)
      (Physics|SetSimulatePhysics (Variables|Character|GetMesh) true))
    (:then_1
      (Utilities|FlowControl|Delay 1.7)
      (Audio|PlaySoundatLocation "/Game/Audio/Grunts-Hits/SC_Death.SC_Death" (Transformation|GetActorLocation) "0, 0, 0" 1.0 1.0 0.0 "/Game/Audio/SA_Character.SA_Character" 0 0 0))))

(event EventBeginPlay)

(event Collision|EventActorBeginOverlap
  (params (OtherActor :type Actor%20Object%20Reference)))

(event EventTick
  (params (DeltaSeconds :type Float%20%28single-precision%29)))

(fn ConstructionScript)

(fn StealthBackAssassin
  (Rendering|SetVisibility (Variables|Default|GetAssassinatePrompt) true false)
  (Animation|PlayAnimMontage "/Game/Characters/RPG_Character/Animations/Assasinations/Paired_Knife_Stealth_KidneyAndNeck_Vic_Montage.Paired_Knife_Stealth_KidneyAndNeck_Vic_Montage" 1.0 "None")
  (CallFunction|Ragdoll)
  (return (Transformation|GetWorldLocation (Variables|Default|GetAssasin%20REF)) (Transformation|GetActorRotation)))