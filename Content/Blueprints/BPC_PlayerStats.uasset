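; Player stats component that tracks health and stamina for BP_ThirdPersonCharacter and mirrors them on its HUD widget.
; It caches the owning character on BeginPlay, and SetupUI fills the initial bars and text.
; Functions decrease, restore (capped at max) or raise the maximum of each stat, each pushing the change straight to the HUD.
; The decrease functions return true once the stat is depleted, though values are not clamped at zero.
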(event Custom|SetupUI
  (bind _playercharacterbp (Variables|Default|GetPlayerCharacterBP))
  (bind _playercharacterbp_2 (Variables|Default|GetPlayerCharacterBP))
  (bind _hud_widget (Variables|/Game/ThirdPerson/Blueprints/BP_ThirdPersonCharacter.BP_ThirdPersonCharacter_C|GetHUD_Widget _playercharacterbp_2))
  (bind _hud_widget_2 (Variables|/Game/ThirdPerson/Blueprints/BP_ThirdPersonCharacter.BP_ThirdPersonCharacter_C|GetHUD_Widget _playercharacterbp))
  ;[0.05098 0.05098 0.05098] Setup UI
  ;;[0.05098 0.05098 0.05098] Setup Stamina Bar
  (Rendering|Components|TextRender|SetText (Variables|/Game/UI/WB_HUD.WB_HUD_C|GetStaminaText _hud_widget_2) (Utilities|Text|ToText(Float) (Variables|Stamina|GetCurrentStamina) "HalfToEven"))
  (Progress|SetPercent (Variables|/Game/UI/WB_HUD.WB_HUD_C|GetStaminaBar _hud_widget_2) (/ (Variables|Stamina|GetCurrentStamina) (Variables|Stamina|GetMaxStamina)))
  ;;[0.05098 0.05098 0.05098] Setup Health Bar
  (Progress|SetPercent (Variables|/Game/UI/WB_HUD.WB_HUD_C|GetHealthBar _hud_widget) (/ (Variables|Health|GetCurrentHealth) (Variables|Health|GetMaxHealth)))
  (Rendering|Components|TextRender|SetText (Variables|/Game/UI/WB_HUD.WB_HUD_C|GetHealthText _hud_widget) (Utilities|Text|ToText(Float) (Variables|Health|GetCurrentHealth) "HalfToEven")))

(event EventBeginPlay
  (bind _asbp_third_person_character (Utilities|Casting|CastToBP_ThirdPersonCharacter (Components|GetOwner)))
  (Variables|Default|SetPlayerCharacterBP _asbp_third_person_character))

(fn DecreaseHealth
  (params (Damage :type Float%20%28double-precision%29))
  (bind _playercharacterbp (Variables|Default|GetPlayerCharacterBP))
  (bind _hud_widget (Variables|/Game/ThirdPerson/Blueprints/BP_ThirdPersonCharacter.BP_ThirdPersonCharacter_C|GetHUD_Widget _playercharacterbp))
  (if (not (<= (Variables|Health|GetCurrentHealth) 0.0))
    (Variables|Health|SetCurrentHealth (- (Variables|Health|GetCurrentHealth) Damage))
    (Rendering|Components|TextRender|SetText (Variables|/Game/UI/WB_HUD.WB_HUD_C|GetHealthText _hud_widget) (Utilities|Text|ToText(Float) (Variables|Health|GetCurrentHealth) "HalfToEven"))
    (Progress|SetPercent (Variables|/Game/UI/WB_HUD.WB_HUD_C|GetHealthBar _hud_widget) (/ (Variables|Health|GetCurrentHealth) (Variables|Health|GetMaxHealth)))
    (if (<= (Variables|Health|GetCurrentHealth) 0.0)
      _
      (else
        (return false))))
  (return true))

(fn IncreaseMaxHealth
  (params (HealhIncrease :type Float%20%28double-precision%29))
  (bind _playercharacterbp (Variables|Default|GetPlayerCharacterBP))
  (bind _hud_widget (Variables|/Game/ThirdPerson/Blueprints/BP_ThirdPersonCharacter.BP_ThirdPersonCharacter_C|GetHUD_Widget _playercharacterbp))
  (Variables|Health|SetMaxHealth (+ HealhIncrease (Variables|Health|GetMaxHealth)))
  (Progress|SetPercent (Variables|/Game/UI/WB_HUD.WB_HUD_C|GetHealthBar _hud_widget) (/ (Variables|Health|GetCurrentHealth) (Variables|Health|GetMaxHealth)))
  (Rendering|Components|TextRender|SetText (Variables|/Game/UI/WB_HUD.WB_HUD_C|GetHealthText _hud_widget) (Utilities|Text|ToText(Float) (Variables|Health|GetCurrentHealth) "HalfToEven")))

(fn DecreaseStamina
  (params (StaminaUsage :type Float%20%28double-precision%29))
  (bind _playercharacterbp (Variables|Default|GetPlayerCharacterBP))
  (bind _hud_widget (Variables|/Game/ThirdPerson/Blueprints/BP_ThirdPersonCharacter.BP_ThirdPersonCharacter_C|GetHUD_Widget _playercharacterbp))
  (if (not (>= 0.0 (Variables|Stamina|GetCurrentStamina)))
    (Variables|Stamina|SetCurrentStamina (- (Variables|Stamina|GetCurrentStamina) StaminaUsage))
    (Rendering|Components|TextRender|SetText (Variables|/Game/UI/WB_HUD.WB_HUD_C|GetStaminaText _hud_widget) (Utilities|Text|ToText(Float) (Variables|Stamina|GetCurrentStamina) "HalfToEven"))
    (Progress|SetPercent (Variables|/Game/UI/WB_HUD.WB_HUD_C|GetStaminaBar _hud_widget) (/ (Variables|Stamina|GetCurrentStamina) (Variables|Stamina|GetMaxStamina)))
    (if (>= 0.0 (Variables|Stamina|GetCurrentStamina))
      _
      (else
        (return false))))
  (return true))

(fn IncreaseMaxStamina
  (params (StaminaIncrease :type Float%20%28double-precision%29))
  (bind _playercharacterbp (Variables|Default|GetPlayerCharacterBP))
  (bind _hud_widget (Variables|/Game/ThirdPerson/Blueprints/BP_ThirdPersonCharacter.BP_ThirdPersonCharacter_C|GetHUD_Widget _playercharacterbp))
  (Variables|Stamina|SetMaxStamina (+ StaminaIncrease (Variables|Stamina|GetMaxStamina)))
  (Rendering|Components|TextRender|SetText (Variables|/Game/UI/WB_HUD.WB_HUD_C|GetStaminaText _hud_widget) (Utilities|Text|ToText(Float) (Variables|Stamina|GetCurrentStamina) "HalfToEven"))
  (Progress|SetPercent (Variables|/Game/UI/WB_HUD.WB_HUD_C|GetStaminaBar _hud_widget) (/ (Variables|Stamina|GetCurrentStamina) (Variables|Stamina|GetMaxStamina))))

(fn IncreaseHealth
  (params (Heal :type Float%20%28double-precision%29))
  (bind _playercharacterbp (Variables|Default|GetPlayerCharacterBP))
  (bind _maxhealth (Variables|Health|GetMaxHealth))
  (bind _hud_widget (Variables|/Game/ThirdPerson/Blueprints/BP_ThirdPersonCharacter.BP_ThirdPersonCharacter_C|GetHUD_Widget _playercharacterbp))
  (Variables|Health|SetCurrentHealth (+ Heal (Variables|Health|GetCurrentHealth)))
  (if (> (Variables|Health|GetCurrentHealth) (Variables|Health|GetMaxHealth))
    (Variables|Health|SetCurrentHealth _maxhealth))
  (Progress|SetPercent (Variables|/Game/UI/WB_HUD.WB_HUD_C|GetHealthBar _hud_widget) (/ (Variables|Health|GetCurrentHealth) _maxhealth))
  (Rendering|Components|TextRender|SetText (Variables|/Game/UI/WB_HUD.WB_HUD_C|GetHealthText _hud_widget) (Utilities|Text|ToText(Float) (Variables|Health|GetCurrentHealth) "HalfToEven")))

(fn IncreaseStamina
  (params (Regen :type Float%20%28double-precision%29))
  (bind _playercharacterbp (Variables|Default|GetPlayerCharacterBP))
  (bind _hud_widget (Variables|/Game/ThirdPerson/Blueprints/BP_ThirdPersonCharacter.BP_ThirdPersonCharacter_C|GetHUD_Widget _playercharacterbp))
  (Variables|Stamina|SetCurrentStamina (+ Regen (Variables|Stamina|GetCurrentStamina)))
  (if (> (Variables|Stamina|GetCurrentStamina) (Variables|Stamina|GetMaxStamina))
    (Variables|Stamina|SetCurrentStamina (Variables|Stamina|GetMaxStamina)))
  (Rendering|Components|TextRender|SetText (Variables|/Game/UI/WB_HUD.WB_HUD_C|GetStaminaText _hud_widget) (Utilities|Text|ToText(Float) (Variables|Stamina|GetCurrentStamina) "HalfToEven"))
  (Progress|SetPercent (Variables|/Game/UI/WB_HUD.WB_HUD_C|GetStaminaBar _hud_widget) (/ (Variables|Stamina|GetCurrentStamina) (Variables|Stamina|GetMaxStamina))))